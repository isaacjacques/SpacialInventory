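; BP_ItemObject is an item data object that exposes an item's dimensions, icon and class.
; It consists of three getters with no other logic.
; GetIcon picks the rotated or standard icon from the Rotated flag, while GetDimensions returns the stored Dimensions without checking that flag.
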(fn `GetDimensions`
  (returns (Dimensions :type "IntPoint Structure"))
  (return (`self.Dimensions`)))

(fn `GetIcon`
  (returns (Icon :type "MaterialInterface Object Reference"))
  (return (select `bool` (`self.Rotated`) :`false` (`self.Icon`) :`true` (`self.IconRotated`))))

(fn `GetItemClass`
  (returns (ItemClass :type "/Game/Items/BP_Item Class Reference"))
  (return (`self.ItemClass`)))