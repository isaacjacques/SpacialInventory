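; Game state Blueprint that provides a helper for spawning an item's world actor in front of a given actor.
; SpawnItemFromActor places the spawn point a short distance along the actor's forward vector, optionally snapping it to the surface below with a downward visibility trace.
; It spawns the class returned by the item object's GetItemClass and passes that item object into the new actor.
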(fn `SpawnItemFromActor`
  (params (Actor :type "Actor Object Reference") (ItemObject :type "/Game/Items/BP_ItemObject Object Reference") (GroundClamp :type Boolean))
  (locals (`SpawnLocation (local)` :type "Vector Structure"))
  (bind _actor (`local.Actor`))
  (bind _itemobject (`local.ItemObject`))
  (`|ExecutionSequence`
    (:`then_0`
      (set `local.SpawnLocation (local)` (+ (`self.K2_GetActorLocation` _actor) (* (`self.GetActorForwardVector` _actor) 150.0)))
      (if (`local.GroundClamp`)
        (bind (_outhit _returnvalue) (`KismetSystemLibrary.LineTraceSingle` (`local.SpawnLocation (local)`) (- (`local.SpawnLocation (local)`) (0.0 0.0 1000.0)) "TraceTypeQuery1"))
        (if _returnvalue
          (set `local.SpawnLocation (local)` (`.Location` (`GameplayStatics.BreakHitResult` _outhit))))))
    (:`then_1`
      (`|SpawnActorFromClass` (`/Game/Items/BP_ItemObject.GetItemClass` _itemobject) (`KismetMathLibrary.MakeTransform` (`local.SpawnLocation (local)`)) "Undefined" "MultiplyWithRoot" null _itemobject null))))

(fn `UserConstructionScript`)